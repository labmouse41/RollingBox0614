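; Beat-timed laser beam hazard that flings BP_CBox actors it touches.
; Ready tracks an in-range target with a thin warning beam for one beat, then locks and fires a thick beam for three beats.
; A separate 4-way mode sweeps the beam on a cosine until deactivated.
; Each tick a line trace sets the beam end, impact effect and stretched overlap capsule, whose hits apply sideways-and-up velocity on the server.
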(event `self.ReceiveBeginPlay`
  (`FXSystemComponent.SetColorParameter` (`self.NiagaraLaser`) "Color" (`self.ReadyColor`))
  (`FXSystemComponent.SetColorParameter` (`self.NiagaraLaserImpact`) "Color" (`self.ReadyColor`))
  (`FXSystemComponent.SetIntParameter` (`self.NiagaraLaserImpact`) "SpawnOn" 0)
  (`KismetSystemLibrary.K2_SetTimerForNextTick` null "SetBeatLength")
  (`PrimitiveComponent.SetCollisionEnabled` (`self.Capsule`) "NoCollision"))

(event `self.ReceiveTick`
  (params (DeltaSeconds :type "Float (single-precision)"))
  (`self.IsAiming` (`self.bAiming`))
  (`self.IsAiming4Way` (`self.bIsAiming4Way`) DeltaSeconds)
  (`self.IsOn` (`self.bLaserTrigger`)))

(event `self.Capsule.OnComponentBeginOverlap`
  (params (OverlappedComponent :type "PrimitiveComponent Object Reference") (OtherActor :type "Actor Object Reference") (OtherComp :type "PrimitiveComponent Object Reference") (OtherBodyIndex :type Integer) (bFromSweep :type Boolean) (SweepResult :type "HitResult Structure (by ref)"))
  (bind _returnvalue (`SceneComponent.GetForwardVector` (`self.Arrow`)))
  ;[1 1 1] Physics
  (`/Engine/EditorBlueprintResources/ActorMacros.Switch Has Authority`
    (:`Authority`
      (bind _asbp_cbox (cast `/Game/GameMode/BP_CBox` OtherActor))
      (`|ExecutionSequence`
        (:`then_0`
          ;[1 1 1] ImpactParticles
          (bind _returnvalue_2 (`NiagaraFunctionLibrary.SpawnSystemAtLocation` "/Game/FX/NG_ParticleOnJump.NG_ParticleOnJump" (`self.K2_GetActorLocation` _asbp_cbox)))
          (`FXSystemComponent.SetIntParameter` _returnvalue_2 "SpawnNumber" 222))
        (:`then_1`
          (`PrimitiveComponent.SetAllPhysicsLinearVelocity` (`BoxCharacter.Cube` _asbp_cbox) (* (`KismetMathLibrary.Normal` (`KismetMathLibrary.VLerp` (`KismetMathLibrary.VLerp` (`KismetMathLibrary.Normal` (`KismetMathLibrary.Cross_VectorVector` _returnvalue (`KismetMathLibrary.Cross_VectorVector` (- (`SceneComponent.K2_GetComponentLocation` OtherComp) (`self.K2_GetActorLocation`)) _returnvalue))) _returnvalue 0.1) (0.0 0.0 1.0) 0.25)) (`self.Power`)) false))))))

(fn `Activate`
  (set `self.bAiming` false)
  (`NiagaraComponent.SetAsset` (`self.NiagaraLaser`) "/Game/FX/NG_LaserThick.NG_LaserThick" true)
  (`FXSystemComponent.SetColorParameter` (`self.NiagaraLaser`) "Color" (`self.ActivatedColor`))
  (`FXSystemComponent.SetIntParameter` (`self.NiagaraLaserImpact`) "SpawnOn" 1)
  (`PrimitiveComponent.SetCollisionEnabled` (`self.Capsule`) "QueryOnly")
  (`KismetSystemLibrary.K2_SetTimer` null "Deactivate" (* 3.0 (`self.BeatLength`))))

(fn `Activate4Way`
  (params (ArrowForwarVector :type "Vector Structure") (ArrowUpVector :type "Vector Structure"))
  (set `self.ArrowForwardVector` ArrowForwarVector)
  (set `self.ArrowUpVector` ArrowUpVector)
  (set `self.Timer44Way` 0.0)
  (set `self.bIsAiming4Way` true)
  (set `self.bLaserTrigger` true)
  (`KismetSystemLibrary.K2_SetTimer` null "Show4WayEffect" 0.2))

(fn `Deactivate`
  (`PrimitiveComponent.SetCollisionEnabled` (`self.Capsule`) "NoCollision")
  (`SceneComponent.SetVisibility` (`self.NiagaraLaser`) false false)
  (`FXSystemComponent.SetIntParameter` (`self.NiagaraLaserImpact`) "SpawnOn" 0)
  (set `self.bLaserTrigger` false))

(fn `Deactivate4Way`
  (set `self.bIsAiming4Way` false)
  (`KismetSystemLibrary.K2_SetTimer` null "Deactivate4Way4Real" (`self.BeatLength`)))

(fn `Deactivate4Way4Real`
  (`PrimitiveComponent.SetCollisionEnabled` (`self.Capsule`) "NoCollision")
  (`SceneComponent.SetVisibility` (`self.NiagaraLaser`) false false)
  (`FXSystemComponent.SetIntParameter` (`self.NiagaraLaserImpact`) "SpawnOn" 0)
  (set `self.bLaserTrigger` false))

(fn `IsAiming`
  (params (Condition :type Boolean))
  (if Condition
    (set `self.LaserEnd` (`self.K2_GetActorLocation` (`self.Target`)))))

(fn `IsAiming4Way`
  (params (Condition :type Boolean) (Timer44Way :type "Float (double-precision)"))
  (bind _returnvalue (`self.K2_GetActorLocation`))
  (bind _returnvalue_2 (* (`self.GetActorForwardVector`) 5555.0))
  (bind _returnvalue_3 (* (`self.GetActorUpVector`) -5555.0))
  (if Condition
    (bind _output_get (set `self.Timer44Way` (+ Timer44Way (`self.Timer44Way`))))
    (if (> _output_get (`self.BeatLength`))
      (set `self.LaserEnd` (+ (`KismetMathLibrary.VLerp` _returnvalue_2 _returnvalue_3 (+ (* (/ (+ (`KismetMathLibrary.FClamp` (* (`KismetMathLibrary.Cos` (* (`self.Timer44Way`) (/ 3.0 (`self.BeatLength`)))) 1.1) -1.0) 1.0) 2.0) -0.5) 0.8)) _returnvalue))
      (else
        (set `self.LaserEnd` (+ (`KismetMathLibrary.VLerp` _returnvalue_2 _returnvalue_3 0.8) _returnvalue))))))

(fn `IsOn`
  (params (Condition :type Boolean))
  (bind _returnvalue (`self.K2_GetActorLocation`))
  (bind _returnvalue_2 (+ _returnvalue (* (`KismetMathLibrary.GetForwardVector` (`KismetMathLibrary.FindLookAtRotation` _returnvalue (`self.LaserEnd`))) 11111.0)))
  (if Condition
    (bind _outhit (`KismetSystemLibrary.LineTraceSingleForObjects` _returnvalue _returnvalue_2 (`|MakeArray` "ObjectTypeQuery1" "ObjectTypeQuery2" "ObjectTypeQuery3" "ObjectTypeQuery4" "ObjectTypeQuery5" "ObjectTypeQuery6" :!type "EObjectTypeQuery Enum") false (`self.Actors2Ignore`)))
    (`|ExecutionSequence`
      (:`then_0`
        (if (`GameplayStatics.BreakHitResult` _outhit)
          (bind _output_get (set `self.LaserEnd` (`.Location` (`GameplayStatics.BreakHitResult` _outhit))))
          (`self.UpdateCollision`)
          (`SceneComponent.K2_SetWorldLocation` (`self.NiagaraLaserImpact`) _output_get false true)
          (if (not (`self.bAiming`))
            (`FXSystemComponent.SetIntParameter` (`self.NiagaraLaserImpact`) "SpawnOn" 1))
          (else
            (`FXSystemComponent.SetIntParameter` (`self.NiagaraLaserImpact`) "SpawnOn" 0)
            (set `self.LaserEnd` _returnvalue_2))))
      (:`then_1`
        (`FXSystemComponent.SetVectorParameter` (`self.NiagaraLaser`) "LaserEnd" (`self.LaserEnd`))
        (`self.UpdateCollision`)))))

(fn `Ready`
  (params (AimTarget :type "Actor Object Reference"))
  (bind _output_get (set `self.LaserEnd` (`self.K2_GetActorLocation` AimTarget)))
  (if (< (`KismetMathLibrary.VSize` (- _output_get (`self.K2_GetActorLocation`))) 6666.0)
    (set `self.Target` AimTarget)
    (set `self.bLaserTrigger` true)
    (set `self.bAiming` true)
    (`FXSystemComponent.SetColorParameter` (`self.NiagaraLaser`) "Color" (`self.ReadyColor`))
    (`NiagaraComponent.SetAsset` (`self.NiagaraLaser`) "/Game/FX/NG_LaserThin.NG_LaserThin" true)
    (`FXSystemComponent.SetIntParameter` (`self.NiagaraLaserImpact`) "SpawnOn" 0)
    (`KismetSystemLibrary.K2_SetTimerForNextTick` null "SetLaserVisibilityOn")
    (`KismetSystemLibrary.K2_SetTimer` null "Activate" (`self.BeatLength`))))

(fn `SetBeatLength`
  (set `self.BeatLength` (`/Game/Blueprints/CPNT_BeatChecker.BeatLength` (`self.CPNT_BeatChecker`))))

(fn `SetLaserVisibilityOn`
  (`SceneComponent.SetVisibility` (`self.NiagaraLaser`) true false))

(fn `Show4WayEffect`
  (`PrimitiveComponent.SetCollisionEnabled` (`self.Capsule`) "QueryOnly")
  (`NiagaraComponent.SetAsset` (`self.NiagaraLaser`) "/Game/FX/NG_LaserThick.NG_LaserThick" true)
  (`self.SetLaserVisibilityOn`)
  (`FXSystemComponent.SetColorParameter` (`self.NiagaraLaser`) "Color" (`self.ActivatedColor`))
  (`FXSystemComponent.SetIntParameter` (`self.NiagaraLaserImpact`) "SpawnOn" 1))

(fn `UpdateCollision`
  (`SceneComponent.K2_SetWorldRotation` (`self.CapsuleHolder`) (`KismetMathLibrary.FindLookAtRotation` (`self.LaserEnd`) (`self.K2_GetActorLocation`)) false false)
  (`SceneComponent.K2_SetWorldLocation` (`self.Capsule`) (`KismetMathLibrary.VLerp` (`self.LaserEnd`) (`self.K2_GetActorLocation`) 0.5) false false)
  (`CapsuleComponent.SetCapsuleHalfHeight` (`self.Capsule`) (* (`KismetMathLibrary.VSize` (- (`self.LaserEnd`) (`self.K2_GetActorLocation`))) 0.5) true))

(fn `UserConstructionScript`)
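; BP_BeatScaler is an actor that pulses the scale of its Cube in time with a beat.
; BeginPlay reads BeatLength from BeatChecker, sets the timeline play rate to its inverse and starts a looping timer at that interval.
; Each timer hit restarts the timeline, whose track drives a uniform world scale offset from one.
; A separate SetBeatLength function, not called here, copies BeatLength from the DontUseMe game mode.
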(event `self.ReceiveBeginPlay`
  ;[1 1 1] BeginPlay
  (`TimelineComponent.SetPlayRate` (`self.타임라인`) (/ 1.0 (`/Game/Blueprints/BeatChecker.BeatLength` (`self.BeatChecker`))))
  (`KismetSystemLibrary.K2_SetTimerDelegate` (delegate `BeatHit`) (`/Game/Blueprints/BeatChecker.BeatLength` (`self.BeatChecker`)) true))

(event `BeatHit`
  (bind (_direction `_새_트랙_0`) (`Timeline|타임라인` :!via `PlayFromStart`)
    (:`Update`
      (`SceneComponent.SetWorldScale3D` (`self.Cube`) (`KismetMathLibrary.Conv_DoubleToVector` (+ (* `_새_트랙_0` 0.5) 1.0))))))

(fn `SetBeatLength`
  (returns (Output_Get :type "Float (double-precision)"))
  (bind _asbp_my_game_mode (cast `/Game/GameMode/DontUseMe` (`GameplayStatics.GetGameMode`)))
  (bind _output_get (set `self.BeatLength` (`/Game/GameMode/DontUseMe.BeatLength` _asbp_my_game_mode)))
  (return _output_get))

(fn `UserConstructionScript`)
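; BP_CubicBlackHole is a paired teleport hazard that captures a box character and spits it out at another black hole.
; On BeginPlay, the authority picks a random other black hole as Exit.
; Overlap starts a pull on the character's cube, intensifies both portals' effects and disables the exit's collision.
; Polling timers wait for BeatChecker.OnBeat to teleport and launch the character randomly, re-enable the exit and calm the effects.
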(event `self.ReceiveBeginPlay`
  ;[1 1 1] SetExit
  (`/Engine/EditorBlueprintResources/ActorMacros.Switch Has Authority`
    (:`Authority`
      (bind _outactors (`GameplayStatics.GetAllActorsOfClass` "BP_CubicBlackHole_C"))
      (bind _output_get (set `self.BlackHoleList` _outactors))
      (`KismetArrayLibrary.Array_RemoveItem` _output_get self)
      (set `self.Exit` (`KismetArrayLibrary.Array_Random` (`self.BlackHoleList`))))))

(event `self.ReceiveTick`
  (params (DeltaSeconds :type "Float (single-precision)"))
  (bind _targetcharacter (`self.TargetCharacter`))
  (if (`self.BlackHoleOn`)
    (`PrimitiveComponent.SetPhysicsLinearVelocity` (`/Game/GameMode/BP_BoxcharacterDontUseMe.Cube` _targetcharacter) (* (`KismetMathLibrary.Normal` (- (`self.K2_GetActorLocation`) (`self.K2_GetActorLocation` _targetcharacter))) (`self.Gravity`) (`GameplayStatics.GetWorldDeltaSeconds`)) true "None")))

(event `PlayEffect`
  (`NiagaraComponent.SetAsset` (`self.NG_PortalSwirlySmoke`) "/Game/FX/NG_PortalFastSwirlySmoke.NG_PortalFastSwirlySmoke" true)
  (`FXSystemComponent.SetFloatParameter` (`self.PortalParticles`) "GravityMultiplier" 222.0)
  (`MeshComponent.SetScalarParameterValueOnMaterials` (`self.InnerRefraction`) "TimeSpeed" 9.0)
  (`KismetSystemLibrary.K2_SetTimer` null "ResetEffectOnBeat" 1.0))

(event `self.Box.OnComponentBeginOverlap`
  (params (OverlappedComponent :type "PrimitiveComponent Object Reference") (OtherActor :type "Actor Object Reference") (OtherComp :type "PrimitiveComponent Object Reference") (OtherBodyIndex :type Integer) (bFromSweep :type Boolean) (SweepResult :type "HitResult Structure (by ref)"))
  (if (`self.IsExit`)
    _
    (elif (not (`self.BlackHoleOn`))
      (bind _asbp_boxcharacter_dont_use_me (cast `/Game/GameMode/BP_BoxcharacterDontUseMe` OtherActor))
      (set `self.TargetCharacter` _asbp_boxcharacter_dont_use_me)
      (`self.PlayEffect`)
      (set `self.BlackHoleOn` true)
      (`self.SetExit`)
      (`KismetSystemLibrary.K2_SetTimer` null "ReleaseOnBeat" 1.0))))

(fn `Release`
  (bind _targetcharacter (`self.TargetCharacter`))
  (`self.SetLocationToExit` (`self.TargetCharacter`) (`self.Exit`))
  (`PrimitiveComponent.SetPhysicsLinearVelocity` (`/Game/GameMode/BP_BoxcharacterDontUseMe.Cube` _targetcharacter) (* (`KismetMathLibrary.RandomUnitVector`) (`self.OutPower`)) false "None")
  (set `/Game/GameMode/BP_BoxcharacterDontUseMe.AirTime` 0.0 _targetcharacter)
  (set `self.BlackHoleOn` false)
  (`KismetSystemLibrary.K2_SetTimer` null "ResetExit" 0.1))

(fn `ReleaseOnBeat`
  (if (`/Game/Blueprints/CPNT_BeatChecker.bOnBeat` (`self.BeatChecker`))
    (`self.Release`)
    (else
      (`KismetSystemLibrary.K2_SetTimer` null "ReleaseOnBeat" 0.05))))

(fn `ResetEffect`
  (`NiagaraComponent.SetAsset` (`self.NG_PortalSwirlySmoke`) "/Game/FX/NG_PortalSlowSwirlySmoke.NG_PortalSlowSwirlySmoke" true)
  (`FXSystemComponent.SetFloatParameter` (`self.PortalParticles`) "GravityMultiplier" 1.0)
  (`MeshComponent.SetScalarParameterValueOnMaterials` (`self.InnerRefraction`) "TimeSpeed" 0.7)
  (`SceneComponent.SetRelativeScale3D` (`self.InnerRefraction`) (0.7 0.7 0.7))
  (`SceneComponent.SetVisibility` (`self.OuterRefraction`) true false))

(fn `ResetEffectOnBeat`
  (if (`/Game/Blueprints/CPNT_BeatChecker.bOnBeat` (`self.BeatChecker`))
    (`self.ResetEffect`)
    (else
      (`KismetSystemLibrary.K2_SetTimer` null "ResetEffectOnBeat" 0.05))))

(fn `ResetExit`
  (bind _exit (`self.Exit`))
  (`PrimitiveComponent.SetCollisionEnabled` (`/Game/Blueprints/BP_CubicBlackHole.Box` _exit) "QueryAndPhysics")
  (set `/Game/Blueprints/BP_CubicBlackHole.BlackHoleOn` false _exit)
  (set `/Game/Blueprints/BP_CubicBlackHole.IsExit` false _exit))

(fn `SetExit`
  (bind _exit (`self.Exit`))
  (`PrimitiveComponent.SetCollisionEnabled` (`/Game/Blueprints/BP_CubicBlackHole.Box` _exit) "NoCollision")
  (set `/Game/Blueprints/BP_CubicBlackHole.IsExit` true _exit)
  (`self.PlayEffect` _exit))

(fn `SetLocationToExit`
  (params (BoxCharacter :type "Actor Object Reference") (Exit :type "Actor Object Reference"))
  (`self.K2_SetActorLocation` BoxCharacter (`self.K2_GetActorLocation` Exit) false true)
  (return))

(fn `UserConstructionScript`
  (locals (NewLocalVar :type "Vector Structure" :default (0.0 0.0 0.0))))
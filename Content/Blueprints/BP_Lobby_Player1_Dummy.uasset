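; Lobby stand-in for Player 1: a cube-based dummy actor moved vertically by a timeline.
; BeginPlay caches the cube's location, then offsets the actor's Z from it by the scaled timeline curve.
; Tick zeroes any linear physics velocity on the cube; a second speed check does nothing.
; SetEdgeGlowColor is called every tick but is empty, with its BeatChecker-driven edge and tail glow logic left disconnected.
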(event `self.ReceiveTick`
  (params (DeltaSeconds :type "Float (single-precision)"))
  ;[1 1 1] Tick
  (`|ExecutionSequence`
    (:`then_0`
      (`self.SetEdgeGlowColor`)
      (bind _returnvalue (`PrimitiveComponent.GetPhysicsLinearVelocity` (`self.Cube`) "None"))
      (if (> (`KismetMathLibrary.VSize` _returnvalue) 0.0)
        (`PrimitiveComponent.SetPhysicsLinearVelocity` (`self.Cube`) (* (0.0 0.0 0.0) (`KismetMathLibrary.Normal` _returnvalue)) false "None")))
    (:`then_1`
      (bind _returnvalue_2 (`PrimitiveComponent.GetPhysicsLinearVelocity` (`self.Cube`) "None"))
      (if (> (`KismetMathLibrary.VSize` _returnvalue_2) 222.0)
        _))))

(event `self.ReceiveBeginPlay`
  (bind _output_get (set `self.CurrentPos` (`SceneComponent.K2_GetComponentLocation` (`self.Cube`))))
  (bind (_direction `_새_트랙_0`) (`Timeline|타임라인_0`)
    (:`Update`
      (`self.K2_SetActorLocation` (`KismetMathLibrary.MakeVector` (.x _output_get) (.y _output_get) (+ (* `_새_트랙_0` 10.0) (.z _output_get)))))))

(fn `SetEdgeGlowColor`)

(fn `UserConstructionScript`)
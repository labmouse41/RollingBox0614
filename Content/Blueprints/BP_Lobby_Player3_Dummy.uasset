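; BP_Lobby_Player3_Dummy is, by its name, a stand-in for the third player in the lobby, built around a physics-driven Cube.
; Each tick clamps the cube's velocity to MaxSpeedByHit, then accumulates AirTime whenever speed exceeds a fixed threshold, without any ground check.
; SetEdgeGlowColor runs each tick but is empty: its beat-driven glow and tail color code is disconnected, as is a timeline that would set the cube's height.
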(event `self.ReceiveTick`
  (params (DeltaSeconds :type "Float (single-precision)"))
  (bind _maxspeedbyhit (`self.MaxSpeedByHit`))
  ;[1 1 1] Tick
  (`|ExecutionSequence`
    (:`then_0`
      (`self.SetEdgeGlowColor`)
      (bind _returnvalue (`PrimitiveComponent.GetPhysicsLinearVelocity` (`self.Cube`) "None"))
      (if (> (`KismetMathLibrary.VSize` _returnvalue) _maxspeedbyhit)
        (`PrimitiveComponent.SetPhysicsLinearVelocity` (`self.Cube`) (* _maxspeedbyhit (`KismetMathLibrary.Normal` _returnvalue)) false "None")))
    (:`then_1`
      (bind _returnvalue_2 (`PrimitiveComponent.GetPhysicsLinearVelocity` (`self.Cube`) "None"))
      (if (> (`KismetMathLibrary.VSize` _returnvalue_2) 222.0)
        (set `self.AirTime` (+ DeltaSeconds (`self.AirTime`)))))))

(event `self.ReceiveBeginPlay`)

(fn `SetEdgeGlowColor`)

(fn `UserConstructionScript`)
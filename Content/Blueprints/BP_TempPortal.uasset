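; BP_TempPortal is a portal effect actor that plays a one-second visual surge when something overlaps its Box; it contains no teleport logic.
; The overlap spikes GravityMultiplier on the core and particle effects and TimeSpeed on InnerRefraction's materials, then lowers both after a delay.
; InnerRefraction gets the same scale in both phases, and OuterRefraction is set visible at the end, as the node that hides it is unwired.
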(event `self.Box.OnComponentBeginOverlap`
  (params (OverlappedComponent :type "PrimitiveComponent Object Reference") (OtherActor :type "Actor Object Reference") (OtherComp :type "PrimitiveComponent Object Reference") (OtherBodyIndex :type Integer) (bFromSweep :type Boolean) (SweepResult :type "HitResult Structure (by ref)"))
  (`FXSystemComponent.SetFloatParameter` (`self.PortalCore`) "GravityMultiplier" 222.0)
  (`FXSystemComponent.SetFloatParameter` (`self.PortalParticles`) "GravityMultiplier" 222.0)
  (`MeshComponent.SetScalarParameterValueOnMaterials` (`self.InnerRefraction`) "TimeSpeed" 9.0)
  (`SceneComponent.SetRelativeScale3D` (`self.InnerRefraction`) (0.4 0.4 0.4))
  (`KismetSystemLibrary.Delay` 1.0)
  (`FXSystemComponent.SetFloatParameter` (`self.PortalCore`) "GravityMultiplier" 1.0)
  (`FXSystemComponent.SetFloatParameter` (`self.PortalParticles`) "GravityMultiplier" 1.0)
  (`MeshComponent.SetScalarParameterValueOnMaterials` (`self.InnerRefraction`) "TimeSpeed" 0.5)
  (`SceneComponent.SetRelativeScale3D` (`self.InnerRefraction`) (0.4 0.4 0.4))
  (`SceneComponent.SetVisibility` (`self.OuterRefraction`) true false))

(fn `UserConstructionScript`)
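; BP_Trem2_Holder is a Blueprint with four trigger zones that launch physics objects entering them.
; Each Collision component's begin-overlap event sets the overlapping component's linear velocity along the forward vector of its matching Arrow component.
; The extremely large velocity replaces the current one rather than adding to it, with no filtering of what overlaps.
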(event `self.Collision_1.OnComponentBeginOverlap`
  (params (OverlappedComponent :type "PrimitiveComponent Object Reference") (OtherActor :type "Actor Object Reference") (OtherComp :type "PrimitiveComponent Object Reference") (OtherBodyIndex :type Integer) (bFromSweep :type Boolean) (SweepResult :type "HitResult Structure (by ref)"))
  (`PrimitiveComponent.SetPhysicsLinearVelocity` OtherComp (* (`SceneComponent.GetForwardVector` (`self.Arrow_1`)) 1000000.0) false "None"))

(event `self.Collision_2.OnComponentBeginOverlap`
  (params (OverlappedComponent :type "PrimitiveComponent Object Reference") (OtherActor :type "Actor Object Reference") (OtherComp :type "PrimitiveComponent Object Reference") (OtherBodyIndex :type Integer) (bFromSweep :type Boolean) (SweepResult :type "HitResult Structure (by ref)"))
  (`PrimitiveComponent.SetPhysicsLinearVelocity` OtherComp (* (`SceneComponent.GetForwardVector` (`self.Arrow_2`)) 1000000.0) false "None"))

(event `self.Collision_3.OnComponentBeginOverlap`
  (params (OverlappedComponent :type "PrimitiveComponent Object Reference") (OtherActor :type "Actor Object Reference") (OtherComp :type "PrimitiveComponent Object Reference") (OtherBodyIndex :type Integer) (bFromSweep :type Boolean) (SweepResult :type "HitResult Structure (by ref)"))
  (`PrimitiveComponent.SetPhysicsLinearVelocity` OtherComp (* (`SceneComponent.GetForwardVector` (`self.Arrow_3`)) 1000000.0) false "None"))

(event `self.Collision_4.OnComponentBeginOverlap`
  (params (OverlappedComponent :type "PrimitiveComponent Object Reference") (OtherActor :type "Actor Object Reference") (OtherComp :type "PrimitiveComponent Object Reference") (OtherBodyIndex :type Integer) (bFromSweep :type Boolean) (SweepResult :type "HitResult Structure (by ref)"))
  (`PrimitiveComponent.SetPhysicsLinearVelocity` OtherComp (* (`SceneComponent.GetForwardVector` (`self.Arrow_4`)) 1000000.0) false "None"))

(fn `UserConstructionScript`)
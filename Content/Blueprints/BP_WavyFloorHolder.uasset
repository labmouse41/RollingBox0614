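; BP_WavyFloorHolder drives a beat-synced floor effect, triggering one random item from its List on every beat.
; On begin play, after a zero-length delay, it starts a looping timer at the BeatChecker's beat length that calls OnBeat.
; OnBeat recursively retries while the random pick is already Triggered, with no guard for all items being triggered.
; The check and the trigger call each read a random item from List.
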(event `self.ReceiveBeginPlay`
  (`KismetSystemLibrary.Delay` 0.0)
  (`self.RepeatOnBeat`))

(event `RepeatOnBeat`
  (`KismetSystemLibrary.K2_SetTimer` null "OnBeat" (`/Game/Blueprints/CPNT_BeatChecker.BeatLength` (`self.BeatChecker`)) true))

(fn `OnBeat`
  (bind _outitem (`KismetArrayLibrary.Array_Random` (`self.List`)))
  (if (`/Game/Blueprints/BP_WavyFloor.bTriggered` _outitem)
    (`self.OnBeat`)
    (else
      (`/Game/Blueprints/BP_WavyFloor.Trigger` _outitem false 0.0))))

(fn `UserConstructionScript`)
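; BP_TeleportAnywhere is a portal that sends an overlapping BP_BoxcharacterDontUseMe to a randomly chosen other portal.
; BeginPlay caches every instance of the class in PortalList.
; On box overlap, RandomEscape removes itself from that list and moves the character's root to a random remaining portal's Scene location, without sweep.
; The Spawn function is an empty stub.
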(event `self.ReceiveBeginPlay`
  (bind _outactors (`GameplayStatics.GetAllActorsOfClass` "BP_TeleportAnywhere_C"))
  (set `self.PortalList` _outactors))

(event `self.Box_0.OnComponentBeginOverlap`
  (params (OverlappedComponent :type "PrimitiveComponent Object Reference") (OtherActor :type "Actor Object Reference") (OtherComp :type "PrimitiveComponent Object Reference") (OtherBodyIndex :type Integer) (bFromSweep :type Boolean) (SweepResult :type "HitResult Structure (by ref)"))
  (`self.RandomEscape` OtherActor))

(fn `RandomEscape`
  (params (Object :type "Object Object Reference"))
  (bind _asbp_boxcharacter (cast `/Game/GameMode/BP_BoxcharacterDontUseMe` Object))
  (`KismetArrayLibrary.Array_RemoveItem` (`self.PortalList`) self)
  (`SceneComponent.K2_SetRelativeLocation` (`Actor.RootComponent` _asbp_boxcharacter) (`SceneComponent.K2_GetComponentLocation` (`/Game/Blueprints/LSJ/BP_TeleportAnywhere.Scene` (`KismetArrayLibrary.Array_Random` (`self.PortalList`)))) false false))

(fn `Spawn`
  (params (BoxCharacter :type "/Game/GameMode/BP_BoxcharacterDontUseMe Object Reference") (Speed :type "Vector Structure"))
  (locals (AfterCharacter :type "/Game/GameMode/BP_BoxcharacterDontUseMe Object Reference") (NewLocalVar_0 :type "Vector Structure" :default (0.0 0.0 0.0))))

(fn `UserConstructionScript`
  (locals (NewLocalVar :type "Vector Structure" :default (0.0 0.0 0.0))))
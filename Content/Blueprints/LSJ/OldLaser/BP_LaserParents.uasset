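; Parent laser obstacle that pushes the box character with a growing force and registers itself in the player's Obstacles array.
; Its mesh starts hidden; a tick counter reveals it after a delay and periodically calls Beam, an empty event here.
; An overlap latches LaserOn, so each tick increases Power and accelerates overlapping characters' cubes along the arrow direction multiplied component-wise by each cube's forward vector.
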(event `self.ReceiveBeginPlay`
  (`SceneComponent.SetVisibility` (`self.LaserMesh`) false false)
  (bind _asbp_boxcharacter (cast `/Game/GameMode/BP_BoxcharacterDontUseMe` (`GameplayStatics.GetPlayerPawn` 0)))
  (bind _output_get (set `/Game/GameMode/BP_BoxcharacterDontUseMe.Obstacles` (`/Game/GameMode/BP_BoxcharacterDontUseMe.Obstacles` _asbp_boxcharacter) _asbp_boxcharacter))
  (`KismetArrayLibrary.Array_Add` _output_get self))

(event `self.ReceiveTick`
  (params (DeltaSeconds :type "Float (single-precision)"))
  (`|ExecutionSequence`
    (:`then_0`
      (set `self.set_Count` (+ (`self.set_Count`) 1))
      (if (== (`self.set_Count`) 30)
        (`SceneComponent.SetVisibility` (`self.LaserMesh`) true false)
        (`self.Beam`)
        (set `self.set_Count` 0)))
    (:`then_1`
      (if (`self.LaserOn`)
        (set `self.Power` (+ 100.0 (`self.Power`)))
        (for _array_element (`PrimitiveComponent.GetOverlappingActors` (`self.LaserMesh`) "/Game/GameMode/BP_BoxcharacterDontUseMe.BP_BoxcharacterDontUseMe_C")
          (bind _asbp_boxcharacter (cast `/Game/GameMode/BP_BoxcharacterDontUseMe` _array_element))
          (bind _cube (`/Game/GameMode/BP_BoxcharacterDontUseMe.Cube` _asbp_boxcharacter))
          (`PrimitiveComponent.AddForce` _cube (* (* (`KismetMathLibrary.Normal` (`SceneComponent.GetForwardVector` (`self.Arrow`))) (`SceneComponent.GetForwardVector` _cube)) (`self.Power`)) "None" true))))))

(event `Beam`)

(event `self.LaserMesh.OnComponentBeginOverlap`
  (params (OverlappedComponent :type "PrimitiveComponent Object Reference") (OtherActor :type "Actor Object Reference") (OtherComp :type "PrimitiveComponent Object Reference") (OtherBodyIndex :type Integer) (bFromSweep :type Boolean) (SweepResult :type "HitResult Structure (by ref)"))
  (if (!= self OverlappedComponent)
    (set `self.LaserOn` true)))

(fn `UserConstructionScript`)
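; Child laser Blueprint, a variant of a laser hazard that fires one sweeping beam and then destroys itself.
; Its Beam event chains three timelines: scale the beam out to LaserLength, sweep the root's pitch through 30 degrees, then animate beam thickness before destroying the actor.
; The final timeline also re-enables player input on every update.
; BeginPlay, Tick and construction defer to the parent.
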(event `self.ReceiveBeginPlay`
  (`parent.ReceiveBeginPlay`))

(event `self.ReceiveTick`
  (params (DeltaSeconds :type "Float (single-precision)"))
  (`parent.ReceiveTick` DeltaSeconds))

(event `self.Beam`
  (bind (_direction `_새_트랙_0`) (`Timeline|타임라인_0`)
    (:`Update`
      (`SceneComponent.K2_SetRelativeTransform` (`self.LaserScene`) (`KismetMathLibrary.MakeTransform` (0.0 0.0 0.0) (struct) (`KismetMathLibrary.MakeVector` 0.5 0.5 (`KismetMathLibrary.Lerp` 0.0 (`self.LaserLength`) `_새_트랙_0`))) false false))
    (:`Finished`
      (bind (_direction_2 `_새_트랙_0_2`) (`Timeline|타임라인_1`)
        (:`Update`
          (`SceneComponent.K2_SetWorldRotation` (`self.DefaultSceneRoot`) (`KismetMathLibrary.MakeRotator` 0.0 (+ (`KismetMathLibrary.Lerp` 0.0 -30.0 `_새_트랙_0_2`) 190.0)) false false))
        (:`Finished`
          (bind (_direction_3 `_새_트랙_0_3`) (`Timeline|타임라인` :!via `PlayFromStart`)
            (:`Update`
              (`self.EnableInput` (`GameplayStatics.GetPlayerPawn` 0) (`GameplayStatics.GetPlayerController` 0))
              (bind _returnvalue (`KismetMathLibrary.Lerp` 0.0 0.5 `_새_트랙_0_3`))
              (`SceneComponent.K2_SetRelativeTransform` (`self.LaserScene`) (`KismetMathLibrary.MakeTransform` (0.0 0.0 0.0) (struct) (`KismetMathLibrary.MakeVector` _returnvalue _returnvalue (`self.LaserLength`))) false false))
            (:`Finished`
              (`self.K2_DestroyActor`))))))))

(fn `UserConstructionScript`
  (`parent.UserConstructionScript`))
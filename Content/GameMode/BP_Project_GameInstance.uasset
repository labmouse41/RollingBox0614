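; Game instance that runs game flow: solo demo start, multiplayer sessions, map travel and menu screens.
; Hosts create a LAN-toggleable session and open the lobby as listen server; clients join found sessions, and server travel changes maps.
; Player profile persists through a SaveGame slot, though the main menu's profile-check call is disconnected.
; Shows main, multiplayer, lobby and game-over widgets, caching the first two, and holds player and lobby names.
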(event `Start_SoloGame`
  (bind _returnvalue (`GameplayStatics.GetPlayerController` 0))
  ;[1 1 1] 게임 솔로 플레이 (DEMO)
  (`GameplayStatics.OpenLevel` "WavyFloor")
  (set `PlayerController.bShowMouseCursor` false _returnvalue)
  (`WidgetBlueprintLibrary.SetInputMode_GameOnly` _returnvalue))

(event `Setup_PlayerName`
  (params (`Player Name` :type Text))
  ;[1 1 1] 플레이어 이름 설정
  (set `self.Player Profile info` (make `/Game/GameMode/SaveData/S_PlayerProfile` `Player Name`))
  (`self.Save Profile`))

(event `Create_MP_Session`
  ;[1 1 1] 멀티플레이 세션 만들기 (SERVER)
  (`CreateSessionCallbackProxy.CreateSession` (`GameplayStatics.GetPlayerController` 0) 4 (`self.IsLan connection`)
    (:`OnSuccess`
      (`self.Set_Player_Name` (`self.Player Name`))
      (`KismetSystemLibrary.PrintString` "Create Session Successfully")
      (`GameplayStatics.OpenLevel` "Lobby_Map" true "listen"))
    (:`OnFailure`
      (`KismetSystemLibrary.PrintString` "Failed to create session -- Gameinstance --"))))

(event `Join_MP_Session`
  (params (`Session Result` :type "BlueprintSessionResult Structure"))
  ;[1 1 1] 멀티플레이 세션에 들어가기 (CLIENT)
  (`JoinSessionCallbackProxy.JoinSession` (`GameplayStatics.GetPlayerController` 0) `Session Result`
    (:`OnSuccess`
      (`self.Set_Player_Name` (`self.Player Name`)))
    (:`OnFailure`
      (`KismetSystemLibrary.PrintString` "Failed to Join session -- Gameinstance --"))))

(event `Travel_To_Map`
  (params (NumOfConnectedPlayer :type Integer) (`Map Name` :type String))
  ;[1 1 1] 레벨 / 세션 이동
  (set `self.Num Of Connected Player` NumOfConnectedPlayer)
  (`KismetSystemLibrary.ExecuteConsoleCommand` (`KismetStringLibrary.Concat_StrStr` "servertravel " `Map Name`) (`GameplayStatics.GetPlayerController` 0)))

(event `UI_Show_Gameover`
  (bind _returnvalue (`GameplayStatics.GetPlayerController` 0))
  ;[1 1 1] Gameover
  (bind _returnvalue_2 (`|CreateWidget` "/Game/Widget/WB_GameOverMenu.WB_GameOverMenu_C"))
  (`UserWidget.AddToViewport` _returnvalue_2 0)
  (set `PlayerController.bShowMouseCursor` true _returnvalue)
  (`WidgetBlueprintLibrary.SetInputMode_UIOnlyEx` _returnvalue null))

(event `UI_Show_Lobby`
  (bind _returnvalue (`GameplayStatics.GetPlayerController` 0))
  ;[1 1 1] 코멘트
  (bind _returnvalue_2 (`|CreateWidget` "/Game/Widget/WB_LobbyMenu.WB_LobbyMenu_C"))
  (`UserWidget.AddToViewport` _returnvalue_2 0)
  (set `PlayerController.bShowMouseCursor` true _returnvalue)
  (`WidgetBlueprintLibrary.SetInputMode_UIOnlyEx` _returnvalue null))

(fn `ChangeConnectionType`
  (returns (IsLanGame :type Boolean))
  (if (`self.IsLan connection`)
    (set `self.IsLan connection` false)
    (else
      (set `self.IsLan connection` true)))
  (return (`self.IsLan connection`)))

(fn `Check for saved Profile`
  (bind _returnvalue (`GameplayStatics.DoesSaveGameExist` (`self.Player Profile Slot`)))
  (if _returnvalue
    (bind _assave_game_player_profile (`self.Load Profile`))
    (set `self.SG_Player profile` _assave_game_player_profile)
    (else
      (`self.Save Profile`)))
  (return))

(fn `get  Lobby Name`
  (returns (`Lobby Name` :type String))
  (return (`self.Lobby Name`)))

(fn `get Booleam Lobby Name Set up`
  (returns (`Lobby Name Bool` :type Boolean))
  (return (`self.Lobby Name Bool`)))

(fn `Get_Player_Name`
  (returns (`Player Name` :type String))
  (return (`self.Player Name`)))

(fn `Load Profile`
  (returns (`AsSave Game Player Profile` :type "/Game/GameMode/SaveData/SaveGame_PlayerProfile Object Reference"))
  (bind _returnvalue (`GameplayStatics.LoadGameFromSlot` (`self.Player Profile Slot`)))
  (bind _assave_game_player_profile (cast `/Game/GameMode/SaveData/SaveGame_PlayerProfile` _returnvalue))
  (set `self.Player Profile info` (`/Game/GameMode/SaveData/SaveGame_PlayerProfile.PlayerProfile` _assave_game_player_profile))
  (return _assave_game_player_profile))

(fn `OnRep_Lobby Name`)

(fn `OnRep_Player Name`)

(fn `Save Profile`
  (bind _sg_player_profile (`self.SG_Player profile`))
  (`/Engine/EditorBlueprintResources/StandardMacros.IsValid` (`self.SG_Player profile`)
    (:`Is Valid`
      _)
    (:`Is Not Valid`
      (bind _returnvalue (`GameplayStatics.CreateSaveGameObject` "/Game/GameMode/SaveData/SaveGame_PlayerProfile.SaveGame_PlayerProfile_C"))
      (set `self.SG_Player profile` _returnvalue)))
  (set `/Game/GameMode/SaveData/SaveGame_PlayerProfile.PlayerProfile` (`self.Player Profile info`) _sg_player_profile)
  (`GameplayStatics.SaveGameToSlot` _sg_player_profile (`self.Player Profile Slot`))
  (return))

(fn `Set Booleam Lobby Name Set up`
  (params (`Lobby Name Bool` :type Boolean))
  (set `self.Lobby Name Bool` `Lobby Name Bool`))

(fn `Set Lobby Name`
  (params (`Lobby Name` :type String))
  (set `self.Lobby Name` `Lobby Name`))

(fn `Set_Player_Name`
  (params (`Player Name` :type String))
  (set `self.Player Name` `Player Name`))

(fn `UI Show Multi Play Session`
  (`/Engine/EditorBlueprintResources/StandardMacros.IsValid` (`self.WB MultiPlay Menu`)
    (:`Is Valid`
      _)
    (:`Is Not Valid`
      (bind _returnvalue (`|CreateWidget` "/Game/Widget/WB_MultiPlay_Menu.WB_MultiPlay_Menu_C" (`GameplayStatics.GetPlayerController` 0)))
      (set `self.WB MultiPlay Menu` _returnvalue)))
  (`UserWidget.AddToViewport` (`self.WB MultiPlay Menu`) 0)
  (return))

(fn `UI_ShowMainmenu`
  (bind _returnvalue (`GameplayStatics.GetPlayerController` 0))
  (`/Engine/EditorBlueprintResources/StandardMacros.IsValid` (`self.WB_Mainmenu`)
    (:`Is Valid`
      _)
    (:`Is Not Valid`
      (bind _returnvalue_2 (`|CreateWidget` "/Game/Widget/WB_Mainmenu.WB_Mainmenu_C" _returnvalue))
      (set `self.WB_Mainmenu` _returnvalue_2)))
  (`UserWidget.AddToViewport` (`self.WB_Mainmenu`) 0)
  (`WidgetBlueprintLibrary.SetInputMode_UIOnlyEx` _returnvalue null)
  (set `PlayerController.bShowMouseCursor` true _returnvalue)
  (return))
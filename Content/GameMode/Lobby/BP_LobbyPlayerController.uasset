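; Lobby player controller that syncs the player's name and handles leaving a network session.
; On possession it chains through ResPosses to read the name from BP_Project_GameInstance and pass it to ReqNewPlayerName, which sets it on BP_LobbyPlayerState.
; EndClientSession destroys the session and then opens MainMenu_Map.
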(event `self.ReceivePossess`
  (params (PossessedPawn :type "Pawn Object Reference"))
  ;[1 1 1] 코멘트
  (`self.ResPosses`))

(event `ResPosses`
  ;[1 1 1] 코멘트
  (bind _asbp_project_game_instance (cast `/Game/GameMode/BP_Project_GameInstance` (`GameplayStatics.GetGameInstance`)))
  (`self.ReqNewPlayerName` (`/Game/GameMode/BP_Project_GameInstance.Get_Player_Name` _asbp_project_game_instance)))

(event `ReqNewPlayerName`
  (params (NewPlayerName :type String))
  ;[1 1 1] 코멘트
  (bind _asbp_lobby_player_state (cast `/Game/GameMode/Lobby/BP_LobbyPlayerState` (`self.PlayerState`)))
  (`/Game/GameMode/Lobby/BP_LobbyPlayerState.Set Player Name` _asbp_lobby_player_state NewPlayerName))

(event `EndClientSession`
  (`DestroySessionCallbackProxy.DestroySession` self
    (:`then`
      (`GameplayStatics.OpenLevel` "MainMenu_Map"))))

(fn `UserConstructionScript`)
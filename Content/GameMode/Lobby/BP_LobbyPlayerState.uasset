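; Lobby player state that holds a replicated player name and notifies the lobby HUD when it changes.
; On BeginPlay it registers itself with the first local player controller's LobbyHud through BindPlayerName.
; SetPlayerName writes the name, and its RepNotify fires the ChangeName dispatcher with an empty string rather than the new name.
; Debug prints trace creation and replication.
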(event `self.ReceiveBeginPlay`
  (bind _aslobby_hud (cast `/Game/GameMode/Lobby/LobbyHud` (`PlayerController.GetHUD` (`GameplayStatics.GetPlayerController` 0))))
  (`/Game/GameMode/Lobby/LobbyHud.Bind Player Name` _aslobby_hud self)
  (`KismetSystemLibrary.PrintString` "Create PlayerState" true true (struct :`G` 0.66 :`B` 1.0 :`A` 1.0) 60.0))

(fn `OnRep_StrPlayerName`
  (`KismetSystemLibrary.PrintString` (`KismetStringLibrary.Concat_StrStr` "-- OnRep PlayerName --" (`self.StrPlayerName`)) true true (struct :`G` 0.66 :`B` 1.0 :`A` 1.0) 60.0)
  (`self.EventDispatcher_ChangeName` ""))

(fn `Set Player Name`
  (params (`Player Name` :type String))
  (set `self.StrPlayerName` `Player Name`))

(fn `UserConstructionScript`)
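; Player-controlled physics cube for multiplayer play, with glowing edges and Niagara tails that react to the music beat.
; Enhanced Input jump and move route through Rep events to Jump and Move, passing camera yaw.
; BeatChecker supplies beat length to materials and tails a tick after BeginPlay, and its OnBeat state drives SetEdgeGlowColor.
; Cube hits fire touch particles scaled by point velocity and airtime, then reset airtime.
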(event `self.ReceiveBeginPlay`
  (`KismetSystemLibrary.K2_SetTimerForNextTick` null "SetBeatLength"))

(event `EnhancedInput|/Game/GameMode/Input/Actions/IA_Jump`
  (params (ActionValue :type Boolean) (ElapsedSeconds :type "Float (double-precision)") (TriggeredSeconds :type "Float (double-precision)") (InputAction :type "InputAction Object Reference" :default "/Game/GameMode/Input/Actions/IA_Jump.IA_Jump"))
  (:`Triggered`
    (`self.RepJump`)))

(event `RepJump`
  (`self.Jump`))

(event `EnhancedInput|/Game/GameMode/Input/Actions/IA_Move`
  (params (ActionValue :type "Vector2D Structure") (ElapsedSeconds :type "Float (double-precision)") (TriggeredSeconds :type "Float (double-precision)") (InputAction :type "InputAction Object Reference" :default "/Game/GameMode/Input/Actions/IA_Move.IA_Move"))
  (bind (_returnvalue_roll _returnvalue_pitch _returnvalue_yaw) (`KismetMathLibrary.BreakRotator` (`Controller.GetControlRotation` (`GameplayStatics.GetPlayerController` 0))))
  (:`Triggered`
    (`self.RepMove` ActionValue_X ActionValue_Y _returnvalue_yaw)))

(event `RepMove`
  (params (ActionValueX :type "Float (double-precision)") (ActionValueY :type "Float (double-precision)") (Yaw :type "Float (double-precision)"))
  (`self.Move` (make `InputActionValue` ActionValueX ActionValueY 0.0 "Axis2D") Yaw))

(event `self.Cube.OnComponentHit`
  (params (HitComponent :type "PrimitiveComponent Object Reference") (OtherActor :type "Actor Object Reference") (OtherComp :type "PrimitiveComponent Object Reference") (NormalImpulse :type "Vector Structure") (Hit :type "HitResult Structure (by ref)"))
  (`self.PlayTouchParticlesOnPoint` Hit_Location (`self.NearestPointAmong8`)))

(fn `PlayTouchParticlesOnPoint`
  (params (PlayLocation :type "Vector Structure") (CheckVelocityHere :type "SceneComponent Object Reference"))
  (bind _returnvalue (* (`self.GetAirTime`) 4.0))
  (bind _returnvalue_2 (* _returnvalue _returnvalue))
  (`SceneComponent.K2_SetWorldLocation` (`self.NG_ParticleOnTouch`) PlayLocation false false)
  (bind _returnvalue_3 (`PrimitiveComponent.GetPhysicsLinearVelocityAtPoint` (`self.Cube`) (`SceneComponent.RelativeLocation` CheckVelocityHere) "None"))
  (`FXSystemComponent.SetVectorParameter` (`self.NG_ParticleOnTouch`) "InheritVelocity" (* _returnvalue_3 0.01))
  (bind _returnvalue_4 (`KismetMathLibrary.Sqrt` (`KismetMathLibrary.VSize` _returnvalue_3)))
  (`FXSystemComponent.SetFloatParameter` (`self.NG_ParticleOnTouch`) "InitialForce" (+ _returnvalue_4 _returnvalue_2))
  (`FXSystemComponent.SetIntParameter` (`self.NG_ParticleOnTouch`) "SpawnNumber" (`KismetMathLibrary.FTrunc` (* (+ _returnvalue_4 (* _returnvalue_2 _returnvalue_2)) 0.1)))
  (`NiagaraComponent.ResetSystem` (`self.NG_ParticleOnTouch`))
  (`self.SetAirTime` 0.0))

(fn `ReqWasdInput`
  (params (ActionValueX1 :type "Float (double-precision)") (ActionValueY1 :type "Float (double-precision)") (ControlRotationRoll1 :type "Float (double-precision)") (ControlRotationYaw1 :type "Float (double-precision)")))

(fn `SetBeatLength`
  (bind _beatlength (`/Game/Blueprints/CPNT_BeatChecker.BeatLength` (`self.BeatChecker`)))
  (`MeshComponent.SetScalarParameterValueOnMaterials` (`self.Cube`) "BeatLength" _beatlength)
  (`FXSystemComponent.SetFloatParameter` (`self.Niagara7`) "BeatLength" _beatlength)
  (`FXSystemComponent.SetFloatParameter` (`self.Niagara6`) "BeatLength" _beatlength)
  (`FXSystemComponent.SetFloatParameter` (`self.Niagara5`) "BeatLength" _beatlength)
  (`FXSystemComponent.SetFloatParameter` (`self.Niagara4`) "BeatLength" _beatlength)
  (`FXSystemComponent.SetFloatParameter` (`self.Niagara3`) "BeatLength" _beatlength)
  (`FXSystemComponent.SetFloatParameter` (`self.Niagara2`) "BeatLength" _beatlength)
  (`FXSystemComponent.SetFloatParameter` (`self.Niagara1`) "BeatLength" _beatlength)
  (`FXSystemComponent.SetFloatParameter` (`self.Niagara`) "BeatLength" _beatlength))

(fn `SetEdgeGlowColor`
  (bind _edgeglowintensity (`self.EdgeGlowIntensity`))
  (bind _returnvalue (`KismetMathLibrary.Conv_BoolToDouble` (`/Game/Blueprints/CPNT_BeatChecker.bOnBeat` (`self.BeatChecker`))))
  (bind _returnvalue_2 (`KismetMathLibrary.LinearColorLerp` (`self.EdgeColor1`) (`self.EdgeColor2`) _returnvalue))
  (`FXSystemComponent.SetColorParameter` (`self.Niagara6`) "Color4Tail" (* _returnvalue_2 (`self.TailGlowIntensity`)))
  (`FXSystemComponent.SetColorParameter` (`self.Niagara`) "Color4Tail" (* _returnvalue_2 (`self.TailGlowIntensity`)))
  (`FXSystemComponent.SetColorParameter` (`self.Niagara2`) "Color4Tail" (* _returnvalue_2 (`self.TailGlowIntensity`)))
  (`FXSystemComponent.SetColorParameter` (`self.Niagara3`) "Color4Tail" (* _returnvalue_2 (`self.TailGlowIntensity`)))
  (`FXSystemComponent.SetColorParameter` (`self.Niagara4`) "Color4Tail" (* _returnvalue_2 (`self.TailGlowIntensity`)))
  (`FXSystemComponent.SetColorParameter` (`self.Niagara5`) "Color4Tail" (* _returnvalue_2 (`self.TailGlowIntensity`)))
  (`FXSystemComponent.SetColorParameter` (`self.Niagara7`) "Color4Tail" (* _returnvalue_2 (`self.TailGlowIntensity`)))
  (`FXSystemComponent.SetColorParameter` (`self.Niagara1`) "Color4Tail" (* _returnvalue_2 (`self.TailGlowIntensity`)))
  (`MeshComponent.SetVectorParameterValueOnMaterials` (`self.Cube`) "EdgeGlowColor" (* (`KismetMathLibrary.Conv_LinearColorToVector` _returnvalue_2) (`KismetMathLibrary.Lerp` _edgeglowintensity (* _edgeglowintensity 3.0) _returnvalue))))

(fn `UserConstructionScript`)
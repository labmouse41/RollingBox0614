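; In-game multiplayer HUD that creates the HUD widget on BeginPlay, adds it to the viewport and switches to game-only input with the cursor hidden.
; BindPlayerState hooks a player state's name-change dispatcher and immediately fires the name-change handler, which refreshes the widget's player list.
; If the widget is not yet valid, the refresh retries itself on a short timer.
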(event `self.ReceiveBeginPlay`
  (bind _returnvalue (`GameplayStatics.GetPlayerController` 0))
  (bind _returnvalue_2 (`|CreateWidget` "/Game/MultiPlay/Widget/HudWidget.HudWidget_C"))
  (bind _output_get (set `self.HudWidget` _returnvalue_2))
  (`UserWidget.AddToViewport` _output_get 0)
  (`self.BindPlayerState` null)
  (`WidgetBlueprintLibrary.SetInputMode_GameOnly` _returnvalue)
  (set `PlayerController.bShowMouseCursor` false _returnvalue))

(fn `BindPlayerState`
  (params (PlayerState :type "/Game/MultiPlay/GameMode/InGame/BP_IngamePlayerState Object Reference"))
  (add `/Game/MultiPlay/GameMode/InGame/BP_IngamePlayerState.EventDispatcher_ChangeName` PlayerState (`|CreateDelegate` :!event `EventChangePlayerName`))
  (`self.EventChangePlayerName` (`/Game/MultiPlay/GameMode/InGame/BP_IngamePlayerState.strPlayerName` PlayerState)))

(fn `EventChangePlayerName`
  (params (PlayerName :type String))
  (`self.UpdatePlayerListHUD`))

(fn `UpdatePlayerListHUD`
  (bind _hudwidget (`self.HudWidget`))
  (`/Engine/EditorBlueprintResources/StandardMacros.IsValid` _hudwidget
    (:`Is Valid`
      (`/Game/MultiPlay/Widget/HudWidget.UpdatePlayerList` _hudwidget))
    (:`Is Not Valid`
      (`KismetSystemLibrary.K2_SetTimer` null "UpdatePlayerListHUD" 0.1))))

(fn `UserConstructionScript`)
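; In-game multiplayer player controller that sets up local input and carries the player's name into the match.
; On BeginPlay, the local controller switches to game-only input and hides the mouse cursor.
; On possess, a chain of custom events reads the name stored in BP_Project_GameInstance and sets it on the BP_LobbyPlayerState.
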(event `self.ReceiveBeginPlay`
  (if (`self.IsLocalPlayerController`)
    (`WidgetBlueprintLibrary.SetInputMode_GameOnly` self)
    (set `self.bShowMouseCursor` false)))

(event `self.ReceivePossess`
  (params (PossessedPawn :type "Pawn Object Reference"))
  (`self.ResPosses`))

(event `ResPosses`
  (bind _asbp_project_game_instance (cast `/Game/GameMode/BP_Project_GameInstance` (`GameplayStatics.GetGameInstance`)))
  (`self.ReqNewPlayerName` (`/Game/GameMode/BP_Project_GameInstance.Get_Player_Name` _asbp_project_game_instance)))

(event `ReqNewPlayerName`
  (params (NewPlayerName :type String))
  (bind _asbp_lobby_player_state (cast `/Game/GameMode/Lobby/BP_LobbyPlayerState` (`self.PlayerState`)))
  (`/Game/GameMode/Lobby/BP_LobbyPlayerState.Set Player Name` _asbp_lobby_player_state NewPlayerName))

(fn `UserConstructionScript`)
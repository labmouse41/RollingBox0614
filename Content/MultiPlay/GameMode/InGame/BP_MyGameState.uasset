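; Multiplayer in-game GameState that keeps a music beat clock and relays player name changes.
; Beat length comes from BPM, and each Tick runs server world time through a cosine with a strictness threshold to open and close the OnBeat window on a shared clock.
; Changes to OnBeat fire an event dispatcher, with a debug print while on beat.
; A player name RepNotify forwards the new name through another dispatcher.
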(event `self.ReceiveBeginPlay`
  (set `self.BeatLength` (/ 60.0 (`self.BPM`))))

(event `self.ReceiveTick`
  (params (DeltaSeconds :type "Float (single-precision)"))
  (bind _returnvalue (!= (`KismetMathLibrary.MapRangeClamped` (`KismetMathLibrary.DegCos` (* (`self.GetServerWorldTimeSeconds`) 360.0 (/ 1.0 (`self.BeatLength`)))) (`self.OnBeatStrictHowMuch`) 1.0 0.0 1.0) 0.0))
  (if (`self.OnBeat`)
    (`KismetSystemLibrary.PrintString` (`KismetStringLibrary.Concat_StrStr` "OnBeat" (`KismetStringLibrary.Conv_DoubleToString` (`self.BeatLength`))) true true (struct :`G` 1.0 :`B` 0.345176 :`A` 1.0) 0.1))
  (if (!= (`self.OnBeat`) _returnvalue)
    (set `self.OnBeat` _returnvalue)
    (`self.EVDSPC_SetOnBeat`)))

(fn `On Rep Str Player Name`
  (`self.EventDispatcher Change Player Name` (`self.Str_Player Name`)))

(fn `OnRep_Str_Player Name`)

(fn `UserConstructionScript`)